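; BP_NewMissile is a homing missile projectile in MechWars that chases a target robot.
; SetTarget stores the robot and, if it is a BP_ThirdPersonCharacter, makes its mesh the ProjectileMovement homing target.
; Tick rotates the missile to face the robot each frame, and the capsule overlap destroys it on touching any BP_ThirdPersonCharacter, with no damage applied here.
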(event OnComponentBeginOverlap(Capsule)
  (params (OverlappedComponent :type Primitive%20Component%20Object%20Reference) (OtherActor :type Actor%20Object%20Reference) (OtherComp :type Primitive%20Component%20Object%20Reference) (OtherBodyIndex :type Integer) (bFromSweep :type Boolean) (SweepResult :type Hit%20Result%20Structure%20%28by%20ref%29))
  (Utilities|Casting|CastToBP_ThirdPersonCharacter OtherActor)
  (Actor|DestroyActor self))

(event Custom|SetTarget
  (params (Robot :type Actor%20Object%20Reference))
  (bind _output_get (Variables|Default|SetRobot Robot))
  (bind _asbp_third_person_character (Utilities|Casting|CastToBP_ThirdPersonCharacter _output_get))
  (Variables|/Script/Engine.ProjectileMovementComponent|SetHomingTargetComponent (Variables|Default|GetProjectileMovement) (Variables|/Script/Engine.Character|GetMesh _asbp_third_person_character)))

(event EventBeginPlay)

(event Collision|EventActorBeginOverlap
  (params (OtherActor :type Actor%20Object%20Reference)))

(event EventTick
  (params (DeltaSeconds :type Float%20%28single-precision%29))
  (Transformation|SetActorRotation (Math|Rotator|FindLookatRotation (Transformation|GetActorLocation) (Transformation|GetActorLocation (Variables|Default|GetRobot)))))

(fn ConstructionScript)