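; Asteroid hazard actor that falls diagonally and explodes on overlapping any actor.
; Tick moves the Cube component a fixed swept step along +Y and down Z, throttled by a Delay on Speed, so larger values mean slower movement.
; Cube overlap calls Kill, which spawns an explosion emitter and destroys the actor after a short delay, and prints a hit message if the other actor is a VRPawn.
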(event OnComponentBeginOverlap(Cube)
  (params (OverlappedComponent :type Primitive%20Component%20Object%20Reference) (OtherActor :type Actor%20Object%20Reference) (OtherComp :type Primitive%20Component%20Object%20Reference) (OtherBodyIndex :type Integer) (bFromSweep :type Boolean) (SweepResult :type Hit%20Result%20Structure%20%28by%20ref%29))
  ;[1 1 1] Hit Logic
  (Utilities|FlowControl|Sequence
    (:then_0
      (CallFunction|Kill))
    (:then_1
      (Utilities|Casting|CastToVRPawn OtherActor)
      (Development|PrintString "YOU GOT HIT"))))

(event Custom|Kill
  (Effects|SpawnEmitteratLocation "/Game/StarterContent/Particles/P_Explosion.P_Explosion" (Transformation|GetWorldLocation (Variables|Default|GetCube)))
  (Utilities|FlowControl|Delay 0.2)
  (Actor|DestroyActor))

(event EventBeginPlay)

(event Collision|EventActorBeginOverlap
  (params (OtherActor :type Actor%20Object%20Reference)))

(event EventTick
  (params (DeltaSeconds :type Float%20%28single-precision%29))
  (bind _cube (Variables|Default|GetCube))
  (bind _returnvalue (Transformation|GetWorldLocation _cube))
  ;[1 1 1] Update Position
  (Utilities|FlowControl|Delay (Variables|Default|Getspeed))
  (Transformation|SetWorldLocation (Variables|Default|GetCube) (Math|Vector|MakeVector (.x _returnvalue) (+ (.y _returnvalue) 5.0) (- (.z _returnvalue) 1e+01)) true false))

(fn ConstructionScript)