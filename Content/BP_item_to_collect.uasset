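; BP_item_to_collect is a collectible item that the VRPawn picks up by overlapping its Trigger component.
; On overlap it destroys itself, then in the same sequence increments the pawn's ItemAmount and calls ItemCollected on its item_Spawner.
; The spawner reference is supplied through the SetItemSpawner event and cast to item_Spawner at pickup.
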(event OnComponentBeginOverlap(trigger)
  (params (OverlappedComponent :type Primitive%20Component%20Object%20Reference) (OtherActor :type Actor%20Object%20Reference) (OtherComp :type Primitive%20Component%20Object%20Reference) (OtherBodyIndex :type Integer) (bFromSweep :type Boolean) (SweepResult :type Hit%20Result%20Structure%20%28by%20ref%29))
  ;[1 1 1] Collision
  (bind _asvrpawn (Utilities|Casting|CastToVRPawn OtherActor))
  (Utilities|FlowControl|Sequence
    (:then_0
      (Actor|DestroyActor))
    (:then_1
      (Default|SetItemAmount _asvrpawn (+ (Variables|/Game/VRTemplate/Blueprints/VRPawn.VRPawn_C|GetitemAmount _asvrpawn) 1))
      (bind _asitem_spawner (Utilities|Casting|CastToitem_Spawner (Variables|Default|GetItemSpawner)))
      (Default|ItemCollected _asitem_spawner))))

(event Custom|SetItemSpawner
  (params (ItemSpawner :type Actor%20Object%20Reference))
  (Variables|Default|SetItemSpawner ItemSpawner))

(fn ConstructionScript)