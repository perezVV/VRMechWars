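; Shop actor that trades the VR pawn's walked distance for items, with a pair of doors tied to a terminal.
; BeginPlay finds a BP_Terminal sharing one of its tags, and Tick hides both doors once that terminal is fixed.
; On trigger overlap, a loop deducts 200 m of DistanceTravelled and adds one item while the balance exceeds 200 m, playing a purchase sound only once.
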(event OnComponentBeginOverlap(trigger)
  (params (OverlappedComponent :type Primitive%20Component%20Object%20Reference) (OtherActor :type Actor%20Object%20Reference) (OtherComp :type Primitive%20Component%20Object%20Reference) (OtherBodyIndex :type Integer) (bFromSweep :type Boolean) (SweepResult :type Hit%20Result%20Structure%20%28by%20ref%29))
  ;[1 1 1] For overlap - checks if the amount is able to be spent, does the distance boost and updates the balance
  (bind _asvrpawn (Utilities|Casting|CastToVRPawn OtherActor))
  (while (> (/ (Variables|/Game/VRTemplate/Blueprints/VRPawn.VRPawn_C|GetdistanceTravelled _asvrpawn) 1e+02) 2e+02)
    (Utilities|FlowControl|Sequence
      (:then_0
        (CallFunction|UpdateWalkingBalance))
      (:then_1
        (CallFunction|ExtraItem))
      (:then_2
        (Utilities|FlowControl|DoOnce false
          (:Completed
            (Audio|PlaySound2D "/Game/SciFiUISounds/Wavs/FX1_6.FX1_6" 1.0 1.0 0.0 0 0)))))))

(event Custom|Update%20Walking%20Balance
  ;[1 1 1] update balance function
  (bind _asvrpawn (Utilities|Casting|CastToVRPawn (Game|Player|GetPlayerPawn 0)))
  (Variables|/Game/VRTemplate/Blueprints/VRPawn.VRPawn_C|SetdistanceTravelled _asvrpawn (- (Variables|/Game/VRTemplate/Blueprints/VRPawn.VRPawn_C|GetdistanceTravelled _asvrpawn) 2e+04)))

(event Custom|Onwatch)

(event Custom|Extra%20Item
  ;[1 1 1] extra item function
  (bind _asvrpawn (Utilities|Casting|CastToVRPawn (Game|Player|GetPlayerPawn 0)))
  (Variables|/Game/VRTemplate/Blueprints/VRPawn.VRPawn_C|SetitemAmount _asvrpawn (+ (Variables|/Game/VRTemplate/Blueprints/VRPawn.VRPawn_C|GetitemAmount _asvrpawn) 1)))

(event EventBeginPlay
  (for _array_element (Variables|Actor|GetTags)
    (bind _output_get (Variables|Default|Settag _array_element))
    (bind _outactors (Actor|GetAllActorsOfClasswithTag "/Game/MechWars/BP_Terminal.BP_Terminal_C" _output_get))
    (for _array_element_2 _outactors
      (Variables|Default|Setterminal _array_element_2))))

(event EventTick
  (params (DeltaSeconds :type Float%20%28single-precision%29))
  ;[1 1 1] to open doors when terminal done
  (bind _asbp_terminal (Utilities|Casting|CastToBP_Terminal (Variables|Default|Getterminal)))
  (if (Variables|/Game/MechWars/BP_Terminal.BP_Terminal_C|GetTerminalFixed _asbp_terminal)
    (Utilities|FlowControl|DoOnce false
      (:Completed
        (Rendering|SetVisibility (Variables|Default|GetL_door) false false)
        (Rendering|SetVisibility (Variables|Default|GetR_door) false false)))))

(fn ConstructionScript)