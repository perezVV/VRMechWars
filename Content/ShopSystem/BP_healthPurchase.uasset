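; BP_healthPurchase is a shop trigger where the VR player buys a full health refill with kill points.
; Overlapping Trigger2 with a VRPawn checks KillPoints against a fixed cost, printing "shoot more" when short.
; On success, UpdateShootingBalance deducts the cost and RefillHealth sets Health to MaxHealth, both acting on player 0's pawn.
; A DoOnce gates the overlap and resets after either outcome, so purchases can repeat.
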(event OnComponentBeginOverlap(trigger2)
  (params (OverlappedComponent :type Primitive%20Component%20Object%20Reference) (OtherActor :type Actor%20Object%20Reference) (OtherComp :type Primitive%20Component%20Object%20Reference) (OtherBodyIndex :type Integer) (bFromSweep :type Boolean) (SweepResult :type Hit%20Result%20Structure%20%28by%20ref%29))
  ;[1 1 1] For overlap - checks if the amount is able to be spent, does the distance boost and updates the balance
  (bind _asvrpawn (Utilities|Casting|CastToVRPawn OtherActor))
  (Utilities|FlowControl|DoOnce false :!label _label
    (:Completed
      (if (>= (Variables|/Game/VRTemplate/Blueprints/VRPawn.VRPawn_C|GetkillPoints _asvrpawn) 5e+02)
        (Utilities|FlowControl|Sequence
          (:then_0
            (CallFunction|UpdateShootingBalance))
          (:then_1
            (CallFunction|RefillHealth)
            (goto _label Reset)))
        (else
          (Development|PrintString "shoot more")
          (goto _label Reset))))))

(event Custom|Refill%20Health
  ;[1 1 1] refill health function
  (bind _asvrpawn (Utilities|Casting|CastToVRPawn (Game|Player|GetPlayerPawn 0)))
  (Variables|/Game/VRTemplate/Blueprints/VRPawn.VRPawn_C|SetHealth _asvrpawn (Variables|/Game/VRTemplate/Blueprints/VRPawn.VRPawn_C|GetMaxHealth _asvrpawn)))

(event Custom|Update%20Shooting%20Balance
  ;[1 1 1] update shoot balance
  (bind _asvrpawn (Utilities|Casting|CastToVRPawn (Game|Player|GetPlayerPawn 0)))
  (Variables|/Game/VRTemplate/Blueprints/VRPawn.VRPawn_C|SetkillPoints _asvrpawn (- (Variables|/Game/VRTemplate/Blueprints/VRPawn.VRPawn_C|GetkillPoints _asvrpawn) 5e+02)))

(event EventBeginPlay)

(event Collision|EventActorBeginOverlap
  (params (OtherActor :type Actor%20Object%20Reference)))

(event EventTick
  (params (DeltaSeconds :type Float%20%28single-precision%29)))

(fn ConstructionScript)