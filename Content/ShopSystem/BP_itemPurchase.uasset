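; Shop pickup actor that sells the player an extra item, paid for with distance walked in VR.
; A sphere overlap, gated by a resettable DoOnce, checks whether the overlapping VRPawn's DistanceTravelled covers the price of 100 metres.
; If so, custom events deduct the distance and increment ItemAmount on player pawn 0.
; Otherwise it prints a "walk more" message.
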(event OnComponentBeginOverlap(sphere)
  (params (OverlappedComponent :type Primitive%20Component%20Object%20Reference) (OtherActor :type Actor%20Object%20Reference) (OtherComp :type Primitive%20Component%20Object%20Reference) (OtherBodyIndex :type Integer) (bFromSweep :type Boolean) (SweepResult :type Hit%20Result%20Structure%20%28by%20ref%29))
  ;[1 1 1] For overlap - checks if the amount is able to be spent, does the distance boost and updates the balance
  (Utilities|FlowControl|DoOnce false :!label _label
    (:Completed
      (bind _asvrpawn (Utilities|Casting|CastToVRPawn OtherActor))
      (if (>= (/ (Variables|/Game/VRTemplate/Blueprints/VRPawn.VRPawn_C|GetdistanceTravelled _asvrpawn) 1e+02) 1e+02)
        (Utilities|FlowControl|Sequence
          (:then_0
            (CallFunction|UpdateBalance))
          (:then_1
            (CallFunction|ExtraItem)
            (goto _label Reset)))
        (else
          (Development|PrintString "walk more")
          (goto _label Reset))))))

(event Custom|Update%20Balance
  ;[1 1 1] update balance function
  (bind _asvrpawn (Utilities|Casting|CastToVRPawn (Game|Player|GetPlayerPawn 0)))
  (Variables|/Game/VRTemplate/Blueprints/VRPawn.VRPawn_C|SetdistanceTravelled _asvrpawn (- (Variables|/Game/VRTemplate/Blueprints/VRPawn.VRPawn_C|GetdistanceTravelled _asvrpawn) 1e+04)))

(event Custom|Onwatch)

(event Custom|Extra%20Item
  ;[1 1 1] extra item function
  (bind _asvrpawn (Utilities|Casting|CastToVRPawn (Game|Player|GetPlayerPawn 0)))
  (Variables|/Game/VRTemplate/Blueprints/VRPawn.VRPawn_C|SetitemAmount _asvrpawn (+ (Variables|/Game/VRTemplate/Blueprints/VRPawn.VRPawn_C|GetitemAmount _asvrpawn) 1)))

(event EventBeginPlay)

(event Collision|EventActorBeginOverlap
  (params (OtherActor :type Actor%20Object%20Reference)))

(event EventTick
  (params (DeltaSeconds :type Float%20%28single-precision%29)))

(fn ConstructionScript)