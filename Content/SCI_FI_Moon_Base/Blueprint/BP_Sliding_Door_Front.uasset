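; BP_Sliding_Door_Front is an automatic two-panel sliding door, from a sci-fi moon base set, that opens on overlap with a Box trigger.
; Overlap begin plays the DoorSlider timeline and overlap end reverses it, with no filtering on the overlapping actor.
; Its Slide track drives lerps of SMDoor01L and SMDoor01R relative locations between Current and New vector variables, which the graphs never set.
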(event OnComponentBeginOverlap(Box)
  (params (OverlappedComponent :type Primitive%20Component%20Object%20Reference) (OtherActor :type Actor%20Object%20Reference) (OtherComp :type Primitive%20Component%20Object%20Reference) (OtherBodyIndex :type Integer) (bFromSweep :type Boolean) (SweepResult :type Hit%20Result%20Structure%20%28by%20ref%29))
  (bind _slide (Timeline|DoorSlider Play)
    (:Update
      (Utilities|FlowControl|Sequence
        (:then_0
          (Transformation|SetRelativeLocation (Variables|Default|GetSM_Door_01_L) (Math|Vector|Lerp(Vector) (Variables|Default|GetCurrent%20Left) (Variables|Default|GetNew%20Left) _slide) false false))
        (:then_1
          (Transformation|SetRelativeLocation (Variables|Default|GetSM_Door_01_R) (Math|Vector|Lerp(Vector) (Variables|Default|GetCurrent%20Right) (Variables|Default|GetNew%20Right) _slide) false false))))))

(event OnComponentEndOverlap(Box)
  (params (OverlappedComponent :type Primitive%20Component%20Object%20Reference) (OtherActor :type Actor%20Object%20Reference) (OtherComp :type Primitive%20Component%20Object%20Reference) (OtherBodyIndex :type Integer))
  (bind _slide (Timeline|DoorSlider Reverse)
    (:Update
      (Utilities|FlowControl|Sequence
        (:then_0
          (Transformation|SetRelativeLocation (Variables|Default|GetSM_Door_01_L) (Math|Vector|Lerp(Vector) (Variables|Default|GetCurrent%20Left) (Variables|Default|GetNew%20Left) _slide) false false))
        (:then_1
          (Transformation|SetRelativeLocation (Variables|Default|GetSM_Door_01_R) (Math|Vector|Lerp(Vector) (Variables|Default|GetCurrent%20Right) (Variables|Default|GetNew%20Right) _slide) false false))))))

(fn ConstructionScript)